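; BP_Player is the player pawn that holds the coin balance and owned item counts for an item shop.
; On BeginPlay it caches the player controller and refreshes coins, updating the main UI and item card buttons on every change.
; Purchases deduct the price, increment the owned count, refresh the card and have the controller spawn the item at a BP_ItemSpawnPoint.
; It also exposes an affordability check and a self-reference getter.
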(event `self.ReceiveBeginPlay`
  (bind _playercontroller (message `/Game/Blueprints/Interfaces/BPI_PlayerController.GetPlayerControllerRef` (`GameplayStatics.GetPlayerController` 0)))
  (set `self.PlayerController` _playercontroller)
  (`self.UpdateAmountOfCoins` 0))

(event `UpdateAmountOfCoins`
  (params (DifferenceValue :type Integer64) (Add :type Boolean))
  ;[1 1 1] 更新所持金钱，传入的Add为true则增加，否则减少
  (bind _output_get (set `self.AmountOfCoins` (select `bool` Add :`false` (- (`self.AmountOfCoins`) DifferenceValue) :`true` (+ (`self.AmountOfCoins`) DifferenceValue))))
  (`/Game/UI/WB_Main.UpdateAmountOfCoins` (`/Game/Blueprints/PC_DungeonClickerController.MainUI` (`self.PlayerController`)) _output_get)
  (`/Game/Blueprints/PC_DungeonClickerController.F_UpdateItemCardButton` (`self.PlayerController`)))

(event `PurchaseItem`
  (params (Item :type "/Game/Blueprints/Structures/ST_ItemInfo Structure") (ItemCard :type "/Game/UI/WB_ItemCard Object Reference"))
  (bind ((`Name_10_44AD7AAF46D6B376B3A649A299E5BC15` _name) (`Price_12_97DDCA48407EE5BA90B76098B4290619` _price)) (break `/Game/Blueprints/Structures/ST_ItemInfo` Item))
  (`self.UpdateAmountOfCoins` (`KismetMathLibrary.Conv_IntToInt64` _price))
  (`BlueprintMapLibrary.Map_Add` (`self.ItemsOwned`) _name (+ (`BlueprintMapLibrary.Map_Find` (`self.ItemsOwned`) _name) 1))
  (`/Game/UI/WB_ItemCard.UpdateItemAmount` ItemCard)
  (bind _returnvalue (`GameplayStatics.GetActorOfClass` "/Game/Blueprints/SpawnPoints/BP_ItemSpawnPoint.BP_ItemSpawnPoint_C"))
  (`/Game/Blueprints/PC_DungeonClickerController.SpawnItem` (`self.PlayerController`) (`.Class_5_6237FBB14BA6F9778170A8840F4C3E1D` (break `/Game/Blueprints/Structures/ST_ItemInfo` Item)) (`self.K2_GetActorLocation` _returnvalue)))

(fn `F_HasEnoughMoney`
  (params (Price :type Integer))
  (returns (Enough :type Boolean))
  (return (<= Price (`self.AmountOfCoins`))))

(fn `GetPlayerPawnRef`
  (returns (PlayerRef :type "/Game/Blueprints/BP_Player Object Reference"))
  (return self))

(fn `UserConstructionScript`)