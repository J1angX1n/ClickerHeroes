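; Blueprint function library of lookup helpers that fetch level, enemy, item and item price rows from their data tables.
; Each function converts its input to a row name and returns the matching row, handling only the Row Found branch.
; Level info is keyed by level, enemy and item info by name after a string Replace, and price by ItemBought plus one.
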(fn `F_GetEnemyInfo`
  (params (EnemyName :type String))
  (returns (EnemyInfo :type "/Game/Blueprints/Structures/ST_EnemyInfo Structure"))
  (bind _returnvalue (`|GetDataTableRow` "/Game/Blueprints/DataTables/DT_EnemyInfo.DT_EnemyInfo" (`KismetStringLibrary.Conv_StringToName` (`KismetStringLibrary.Replace` EnemyName " ")))
    (:`then`
      (return _returnvalue))))

(fn `F_GetItemInfo`
  (params (ItemName :type String))
  (returns (ItemInfo :type "/Game/Blueprints/Structures/ST_ItemInfo Structure"))
  (bind _returnvalue (`|GetDataTableRow` "/Game/Blueprints/DataTables/DT_ItemInfo.DT_ItemInfo" (`KismetStringLibrary.Conv_StringToName` (`KismetStringLibrary.Replace` ItemName " ")))
    (:`then`
      (return _returnvalue))))

(fn `F_GetItemPrice`
  (params (ItemBought :type Integer))
  (returns (ItemPrice :type "/Game/Blueprints/Structures/ST_ItemPrice Structure"))
  (bind _returnvalue (`|GetDataTableRow` "/Game/Blueprints/DataTables/DT_ItemPrice.DT_ItemPrice" (`KismetStringLibrary.Conv_StringToName` (`KismetStringLibrary.Conv_IntToString` (+ ItemBought 1))))
    (:`then`
      (return _returnvalue))))

(fn `F_GetLevelInfo`
  (params (Level :type Integer))
  (returns (LevelInfo :type "/Game/Blueprints/Structures/ST_LevelInfo Structure"))
  (bind _returnvalue (`|GetDataTableRow` "/Game/Blueprints/DataTables/DT_LevelInfo.DT_LevelInfo" (`KismetStringLibrary.Conv_StringToName` (`KismetStringLibrary.Conv_IntToString` Level)))
    (:`then`
      (return _returnvalue))))