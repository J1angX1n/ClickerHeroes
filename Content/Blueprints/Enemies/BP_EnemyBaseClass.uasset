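; Base enemy for a dungeon clicker: a flipbook-animated character that takes the player's click damage and advances the game mode to the next level on death.
; GetEnemyInfo, keyed by name, supplies health and idle, hit and death animations.
; Clicking the capsule applies damage, plays the hit animation and spawns a controller effect; damage updates the health bar widget.
; Zero health sets IsDead, which Tick polls to run the death sequence.
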(event `self.ReceiveBeginPlay`
  (bind _gamemoderef (message `/Game/Blueprints/Interfaces/BPI_GameModeBase.GetGameModeRef` (`GameplayStatics.GetGameMode`)))
  (set `self.Game Mode Ref` _gamemoderef)
  (bind _playerref (message `/Game/Blueprints/Interfaces/BPI_PlayerPawnBase.GetPlayerPawnRef` (`GameplayStatics.GetPlayerPawn` 0)))
  (set `self.Player Ref` _playerref)
  (bind _aswb_enemy_health_bar (cast `/Game/UI/WB_EnemyHealthBar` (`WidgetComponent.GetUserWidgetObject` (`self.EnemyInfoWidget`))))
  (`/Game/UI/WB_EnemyHealthBar.ShowEnemyInfo` _aswb_enemy_health_bar (`self.Name`) (`/Game/Blueprints/GM_DungeonClicker.Level` (`self.Game Mode Ref`)))
  (set `self.EnemyHealth` (`.Health_14_ADD3D8A34B2BDCB64D4ACCA0AF90D87C` (break `/Game/Blueprints/Structures/ST_EnemyInfo` (`/Game/Blueprints/Libraries/BP_BPFunctionLibraries.GetEnemyInfo` (`self.Name`)))))
  (`self.UpdateHealth`))

(event `self.ReceiveTick`
  (params (DeltaSeconds :type "Float (single-precision)"))
  (if (`self.IsDead`)
    (`self.OnEnemyDie`)))

(event `self.CapsuleComponent.OnClicked`
  (params (TouchedComponent :type "PrimitiveComponent Object Reference") (ButtonPressed :type "Key Structure"))
  (if (not (`self.IsDead`))
    (`GameplayStatics.ApplyDamage` self (`/Game/Blueprints/BP_Player.ClickDamage` (`self.Player Ref`)))
    (`self.OnHit`)
    (bind _asdungeon_clicker (cast `/Game/Blueprints/PC_DungeonClicker` (`GameplayStatics.GetPlayerController` 0)))
    (`/Game/Blueprints/PC_DungeonClicker.SpawnHitEffect` _asdungeon_clicker)))

(event `self.ReceiveAnyDamage`
  (params (Damage :type "Float (single-precision)") (DamageType :type "DamageType Object Reference") (InstigatedBy :type "Controller Object Reference") (DamageCauser :type "Actor Object Reference"))
  (set `self.EnemyHealth` (`KismetMathLibrary.FClamp` (- (`self.EnemyHealth`) Damage) 0.0 (`self.EnemyHealth`)))
  (`self.UpdateHealth`))

(event `UpdateHealth`
  (bind _aswb_enemy_health_bar (cast `/Game/UI/WB_EnemyHealthBar` (`WidgetComponent.GetUserWidgetObject` (`self.EnemyInfoWidget`))))
  (`/Game/UI/WB_EnemyHealthBar.UpdateHeathInfo` _aswb_enemy_health_bar (`self.EnemyHealth`) (`.Health_14_ADD3D8A34B2BDCB64D4ACCA0AF90D87C` (break `/Game/Blueprints/Structures/ST_EnemyInfo` (`/Game/Blueprints/Libraries/BP_BPFunctionLibraries.GetEnemyInfo` (`self.Name`)))))
  (if (== (`self.EnemyHealth`) 0.0)
    (set `self.IsDead` true)))

(event `OnHit`
  (`PaperFlipbookComponent.SetFlipbook` (`self.Sprite`) (`.HitAnim_21_047F2DF44CAEBEB6420DA2976C41A4AE` (break `/Game/Blueprints/Structures/ST_EnemyInfo` (`/Game/Blueprints/Libraries/BP_BPFunctionLibraries.GetEnemyInfo` (`self.Name`)))))
  (`KismetSystemLibrary.Delay` (`PaperFlipbookComponent.GetFlipbookLength` (`self.Sprite`)))
  (`PaperFlipbookComponent.SetFlipbook` (`self.Sprite`) (`.IdleAnim_20_DD6159D64FDAD84815F03BAD482D9FEA` (break `/Game/Blueprints/Structures/ST_EnemyInfo` (`/Game/Blueprints/Libraries/BP_BPFunctionLibraries.GetEnemyInfo` (`self.Name`))))))

(event `OnEnemyDie`
  (`PaperFlipbookComponent.SetFlipbook` (`self.Sprite`) (`.DeathAnim_22_6B08069941D1CED2AC1C11BCE0C40D89` (break `/Game/Blueprints/Structures/ST_EnemyInfo` (`/Game/Blueprints/Libraries/BP_BPFunctionLibraries.GetEnemyInfo` (`self.Name`)))))
  (`PaperFlipbookComponent.SetLooping` (`self.Sprite`) false)
  (`KismetSystemLibrary.Delay` (`PaperFlipbookComponent.GetFlipbookLength` (`self.Sprite`)))
  (`self.K2_DestroyActor`)
  (`/Game/Blueprints/GM_DungeonClicker.GoNextLevel` (`self.Game Mode Ref`)))

(fn `UserConstructionScript`)