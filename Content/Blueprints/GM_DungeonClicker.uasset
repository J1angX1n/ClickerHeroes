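; Game mode for a dungeon clicker that runs level progression, enemy spawning and a timed round.
; It looks up each level's enemy class and has the player controller spawn it at an enemy point actor, with GoNextLevel advancing up to a maximum level.
; A looping timer counts the round down into the main UI, restoring the enemy's health and resetting the clock when time runs out.
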(event `self.ReceiveBeginPlay`
  (bind _returnvalue (`GameplayStatics.GetActorOfClass` "/Game/Blueprints/SpawnPoints/BP_EnemyPoint1.BP_EnemyPoint1_C"))
  (set `self.EnemyPoint` _returnvalue)
  (bind _aspc_dungeon_clicker_controller (cast `/Game/Blueprints/PC_DungeonClickerController` (`GameplayStatics.GetPlayerController` 0)))
  (bind _output_get (set `self.PlayerController` _aspc_dungeon_clicker_controller))
  (`/Game/Blueprints/PC_DungeonClickerController.SpawnEnemy` _output_get (`.Class_23_D7DC13204B2BF5BA333358B35036F107` (break `/Game/Blueprints/Structures/ST_EnemyInfo` (`/Game/Blueprints/Libraries/BP_BPFunctionLibraries.GetEnemyInfo` (`.EnemyName_7_0323E6F048F23F45A96ADE8109160AD7` (break `/Game/Blueprints/Structures/ST_LevelInfo` (`/Game/Blueprints/Libraries/BP_BPFunctionLibraries.GetLevelInfo` (`self.Level`))))))) (`self.GetTransform` (`self.EnemyPoint`)))
  (`self.StartRoundTimer`))

(event `GoNextLevel`
  ;[1 1 1] 开启下一关
  (if (< (`self.Level`) (`self.MaxLevel`))
    (`/Engine/EditorBlueprintResources/StandardMacros.IncrementInt` (`self.Level`)
      (:`  `
        (`/Game/Blueprints/PC_DungeonClickerController.SpawnEnemy` (`self.PlayerController`) (`self.GetEnemyToSpawn`) (`self.GetTransform` (`self.EnemyPoint`)))
        (`self.StartRoundTimer`)))))

(event `StartRoundTimer`
  (set `self.CurrentTime` (`self.InitialTime`))
  (bind _returnvalue (`KismetSystemLibrary.K2_SetTimerDelegate` (delegate `RoundTimerLoop`) (`self.TimeInterval`) true))
  (set `self.RoundTImeHandle` _returnvalue))

(event `RoundTimerLoop`
  (bind _output_get (set `self.CurrentTime` (`KismetMathLibrary.FClamp` (- (`self.CurrentTime`) (`self.TimeInterval`)) 0.0 (`self.InitialTime`))))
  (`/Game/UI/WB_Main.UpdateRoundTimer` (`/Game/Blueprints/PC_DungeonClickerController.MainUI` (`self.PlayerController`)) _output_get)
  (if (== (`self.CurrentTime`) 0.0)
    (`/Game/Blueprints/Enemies/BP_EnemyBaseClass.RestoreHealth` (`/Game/Blueprints/PC_DungeonClickerController.SpawnedEnemy` (`self.PlayerController`)))
    (set `self.CurrentTime` (`self.InitialTime`))))

(fn `GetEnemyToSpawn`
  (returns (Class :type "/Game/Blueprints/Enemies/BP_EnemyBaseClass Class Reference"))
  (return (`.Class_23_D7DC13204B2BF5BA333358B35036F107` (break `/Game/Blueprints/Structures/ST_EnemyInfo` (`/Game/Blueprints/Libraries/BP_BPFunctionLibraries.GetEnemyInfo` (`.EnemyName_7_0323E6F048F23F45A96ADE8109160AD7` (break `/Game/Blueprints/Structures/ST_LevelInfo` (`/Game/Blueprints/Libraries/BP_BPFunctionLibraries.GetLevelInfo` (`self.Level`)))))))))

(fn `GetGameModeRef`
  (returns (GameModeRef :type "/Game/Blueprints/GM_DungeonClicker Object Reference"))
  (return self))

(fn `UserConstructionScript`)