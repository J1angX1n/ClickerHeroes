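; Player controller for a dungeon clicker game that builds the UI and spawns enemies, hit effects and damage text.
; On BeginPlay it creates the main screen, item cards from DT_ItemInfo, a tooltip, a level-switch card and a custom cursor driven by Enhanced Input clicks.
; Buy buttons are colored and enabled by comparing item prices against the pawn's coins.
; Main and Ascension widgets are created lazily, and effects spawn at the deprojected mouse position.
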(event `self.ReceiveBeginPlay`
  (bind _playerref (message `/Game/Blueprints/Interfaces/BPI_PlayerPawnBase.GetPlayerPawnRef` (`GameplayStatics.GetPlayerPawn` 0)))
  (set `self.PlayerPawn` _playerref)
  (`self.ShowHideWidget` "NewEnumerator0" true)
  (`self.CreateItemCards`)
  (`self.DisplayItemCards`)
  (`self.F_UpdateItemCardButton`)
  (`self.InitializeToolTip`)
  (`self.AddSwitchLevelCard` 1)
  (`self.CreateMouseCursor`)
  (`EnhancedInputSubsystemInterface.AddMappingContext` (subsystem `EnhancedInputLocalPlayerSubsystem`) "/Game/Blueprints/Inputs/IMC_MouseClick.IMC_MouseClick" 0 (struct)))

(event `SpawnEnemy`
  (params (Class :type "Actor Class Reference") (SpawnTransfrom :type "Transform Structure"))
  ;[1 1 1] 生成敌人
  (bind _returnvalue (`|SpawnActorFromClass` Class SpawnTransfrom "Undefined" "MultiplyWithRoot" null null))
  (bind _enemyref (message `/Game/Blueprints/Interfaces/BPI_EnemyBase.GetEnemyRef` _returnvalue))
  (set `self.SpawnedEnemy` _enemyref))

(event `EnhancedInput|/Game/Blueprints/Inputs/IA_MouseClick`
  (params (ActionValue :type Boolean) (ElapsedSeconds :type "Float (double-precision)") (TriggeredSeconds :type "Float (double-precision)") (InputAction :type "InputAction Object Reference" :default "/Game/Blueprints/Inputs/IA_MouseClick.IA_MouseClick"))
  (:`Triggered`
    (`/Game/UI/WB_MouseCursor.SetMouseState` (`self.MouseCursor`) "NewEnumerator1"))
  (:`Completed`
    (`/Game/UI/WB_MouseCursor.SetMouseState` (`self.MouseCursor`) "NewEnumerator0")))

(event `SpawnHitEffect`
  ;[1 1 1] 生成攻击特效
  (`|SpawnActorFromClass` "/Game/Blueprints/BP_HitEffectActor.BP_HitEffectActor_C" (`KismetMathLibrary.Conv_VectorToTransform` (- (`self.DeprojectMousePositionToWorld`) (0.0 1.0 0.0))) "DontSpawnIfColliding" "MultiplyWithRoot" null null))

(event `SpawnDamageText`
  (params (Damage :type Text))
  ;[1 1 1] 生成伤害数字
  (`|SpawnActorFromClass` "/Game/Blueprints/BP_DamageTextActor.BP_DamageTextActor_C" (`KismetMathLibrary.Conv_VectorToTransform` (- (`self.DeprojectMousePositionToWorld`) (0.0 1.0 0.0))) "Undefined" "MultiplyWithRoot" null Damage null))

(event `ShowHideWidget`
  (params (Widget :type "/Game/Blueprints/Enums/E_GameWidgets Enum" :default "NewEnumerator0") (Show :type Boolean))
  ;[1 1 1] 控制主界面的显示/隐藏
  (if Show
    (`self.F_ShowWidget` Widget)
    (else
      (`self.F_HideWidget` Widget))))

(event `CreateItemCards`
  ;[1 1 1] 创建道具
  (`KismetArrayLibrary.Array_Clear` (`self.ItemCards`))
  (bind _outrownames (`DataTableFunctionLibrary.GetDataTableRowNames` "/Game/Blueprints/DataTables/DT_ItemInfo.DT_ItemInfo"))
  (for _array_element _outrownames
    (bind _iteminfo (`/Game/Blueprints/Libraries/BP_BPFunctionLibraries.F_GetItemInfo` (`KismetStringLibrary.Conv_NameToString` _array_element)))
    (bind _returnvalue (`|CreateWidget` "/Game/UI/WB_ItemCard.WB_ItemCard_C" null _iteminfo))
    (`KismetArrayLibrary.Array_Add` (`self.ItemCards`) _returnvalue)))

(event `DisplayItemCards`
  ;[1 1 1] 将道具显示到UI
  (`PanelWidget.ClearChildren` (`/Game/UI/WB_Main.VB_ItemVerticalBox` (`self.MainUI`)))
  (for _array_element (`self.ItemCards`)
    (`PanelWidget.AddChild` (`/Game/UI/WB_Main.VB_ItemVerticalBox` (`self.MainUI`)) _array_element)))

(event `InitializeToolTip`
  ;[1 1 1] 显示购买时悬浮提示
  (bind _returnvalue (`|CreateWidget` "/Game/UI/WB_DamageToolTip.WB_DamageToolTip_C"))
  (set `self.ToolTip` _returnvalue))

(event `AddSwitchLevelCard`
  (params (level :type Integer))
  ;[1 1 1] 添加关卡切换按钮
  (bind _returnvalue (`|CreateWidget` "/Game/UI/WB_SwitchLevel.WB_SwitchLevel_C" null level))
  (`VerticalBox.AddChildToVerticalBox` (`/Game/UI/WB_Main.VB_LevelVerticalBox` (`self.MainUI`)) _returnvalue))

(event `CreateMouseCursor`
  ;[1 1 1] 创建鼠标图片
  (bind _returnvalue (`|CreateWidget` "/Game/UI/WB_MouseCursor.WB_MouseCursor_C"))
  (bind _output_get (set `self.MouseCursor` _returnvalue))
  (`self.SetMouseCursorWidget` "Default" _output_get))

(fn `F_HideWidget`
  (params (Widget :type "/Game/Blueprints/Enums/E_GameWidgets Enum" :default "NewEnumerator0"))
  (switch `/Game/Blueprints/Enums/E_GameWidgets` Widget
    (:`NewEnumerator0`
      (bind _mainui (`self.MainUI`)
        (:`then`
          (`Widget.RemoveFromParent` _mainui))
        (:`else`)))
    (:`NewEnumerator1`
      (bind _ascensionpopup (`self.AscensionPopUp`)
        (:`then`
          (`Widget.RemoveFromParent` _ascensionpopup))
        (:`else`)))))

(fn `F_ShowWidget`
  (params (Widget :type "/Game/Blueprints/Enums/E_GameWidgets Enum" :default "NewEnumerator0"))
  (switch `/Game/Blueprints/Enums/E_GameWidgets` Widget
    (:`NewEnumerator0`
      (`self.MainUI`
        (:`then`
          _)
        (:`else`
          (bind _returnvalue (`|CreateWidget` "/Game/UI/WB_Main.WB_Main_C"))
          (bind _output_get (set `self.MainUI` _returnvalue))))
      (`UserWidget.AddToViewport` _output_get 0))
    (:`NewEnumerator1`
      (`self.AscensionPopUp`
        (:`then`
          _)
        (:`else`
          (bind _returnvalue_2 (`|CreateWidget` "/Game/UI/WB_AscensionPopUp.WB_AscensionPopUp_C"))
          (bind _output_get_2 (set `self.AscensionPopUp` _returnvalue_2))))
      (`UserWidget.AddToViewport` _output_get_2 0))))

(fn `F_UpdateItemCardButton`
  (for _array_element (`self.ItemCards`)
    (bind _returnvalue (> (`/Game/Blueprints/BP_Player.F_GetItemPrice` (`self.PlayerPawn`) (`/Game/UI/WB_ItemCard.ItemInfo` _array_element)) (`/Game/Blueprints/BP_Player.AmountOfCoins` (`self.PlayerPawn`))))
    (`TextBlock.SetColorAndOpacity` (`/Game/UI/WB_ItemCard.TXT_Buy` _array_element) (make `SlateColor` (`KismetMathLibrary.SelectColor` (struct :`R` 0.732639 :`G` 0.082198 :`A` 1.0) (struct :`R` 0.388235 :`G` 1.0 :`B` 0.203922 :`A` 1.0) _returnvalue)))
    (`Widget.SetIsEnabled` (`/Game/UI/WB_ItemCard.Btn_Buy` _array_element) (not _returnvalue))))

(fn `GetPlayerControllerRef`
  (returns (PlayerController :type "/Game/Blueprints/PC_DungeonClickerController Object Reference"))
  (return self))

(fn `UserConstructionScript`)